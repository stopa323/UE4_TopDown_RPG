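; BP_MoveIndicator is a short-lived visual indicator actor, apparently for movement feedback, that shrinks and then removes itself.
; BeginPlay starts a timer from LifetimeTimer that calls DestroyIndicator to destroy the actor, and copies that duration into Lifetime.
; Tick subtracts delta time over Lifetime from the Scene component's world scale, a linear shrink that reaches zero at expiry only from unit scale.
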(event EventTick
  (params (DeltaSeconds :type Float%20%28single-precision%29))
  ;[1 1 1] Smoothly decrease size of indicator
  (Transformation|SetWorldScale3D (Variables|Default|GetScene) (- (Transformation|GetWorldScale (Variables|Default|GetScene)) (/ DeltaSeconds (Variables|Default|Getlifetime_)))))

(event EventBeginPlay
  (bind _lifetime_timer_ (Variables|Default|Getlifetime_timer_))
  ;[1 1 1] Set destroy timer
  (Utilities|Time|SetTimerbyFunctionName self "DestroyIndicator" _lifetime_timer_)
  (Variables|Default|Setlifetime_ _lifetime_timer_))

(fn ConstructionScript)

(fn DestroyIndicator
  (Actor|DestroyActor))