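; Player character ability manager that creates and drives the Blink ability.
; On BeginPlay it spawns an Abb_Blink actor and keeps the reference.
; An activation event forwards an input struct to Blink and prints the result.
; UpdateAbbilities passes delta time to Blink so it can update its timers.
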(event Custom|EActivateBlink
  (params (inInputStruct :type S%20Abbility%20Input%20Object%20Reference%20%28by%20ref%29))
  (bind _outactivated (Default|Activate (Variables|Abbilities|GetBlink) inInputStruct))
  (Development|PrintString (Utilities|String|ToString(Boolean) _outactivated)))

(event EventBeginPlay
  (Utilities|InitializeAbbilities))

(fn ConstructionScript)

(fn UpdateAbbilities
  (params (inDelta :type Float%20%28single-precision%29))
  (Default|UpdateTimers (Variables|Abbilities|GetBlink) inDelta))