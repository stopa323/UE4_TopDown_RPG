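; Blink ability that teleports the input struct's pawn toward a requested destination, capped by Range.
; Activate runs the parent activation, then casts the input to SBlinkInput, printing an error if that fails.
; In-range blinks land on the destination; longer ones use the normalized direction times Range as the absolute location, without adding the pawn's position.
; Both teleports pass zero rotation; feasibility and timer updates defer to the parent.
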(fn ConstructionScript
  (|CallParentFunction))

(fn IsActivateFeasible
  (params (inInputStruct :type S%20Abbility%20Input%20Object%20Reference%20%28by%20ref%29))
  (bind _outpossible (|CallParentFunction inInputStruct))
  (return _outpossible))

(fn Activate
  (params (inInputStruct :type S%20Abbility%20Input%20Object%20Reference%20%28by%20ref%29))
  ;[1 1 1] Derived IsActivateFeasible called here
  (bind _outactivated (|CallParentFunction inInputStruct))
  ;[0 0 0] if true, ready for further poscessing
  (if _outactivated
    (bind _assblink_input (Utilities|Casting|CastToSBlinkInput inInputStruct)
      (:then
        ;[0 0 0] if range exceeded try to blink as fas as possible in that direction
        (if (> (Math|Vector|VectorLength (- (Variables|/Game/GameContent/Blueprints/Abbilities/AbbilityInputData/SBlinkInput.SBlinkInput_C|Getblink_destination_ _assblink_input) (Transformation|GetActorLocation (Variables|/Game/GameContent/Blueprints/Abbilities/AbbilityInputData/SBlinkInput.SBlinkInput_C|Getpawn_ _assblink_input)))) (Variables|Default|Getrange_))
          (bind _returnvalue (Transformation|Teleport (Variables|/Game/GameContent/Blueprints/Abbilities/AbbilityInputData/SBlinkInput.SBlinkInput_C|Getpawn_ _assblink_input) (* (Math|Vector|Normalize (- (Variables|/Game/GameContent/Blueprints/Abbilities/AbbilityInputData/SBlinkInput.SBlinkInput_C|Getblink_destination_ _assblink_input) (Transformation|GetActorLocation (Variables|/Game/GameContent/Blueprints/Abbilities/AbbilityInputData/SBlinkInput.SBlinkInput_C|Getpawn_ _assblink_input)))) (Variables|Default|Getrange_)) "0, 0, 0"))
          (return _returnvalue)
          (else
            (bind _returnvalue_2 (Transformation|Teleport (Variables|/Game/GameContent/Blueprints/Abbilities/AbbilityInputData/SBlinkInput.SBlinkInput_C|Getpawn_ _assblink_input) (Variables|/Game/GameContent/Blueprints/Abbilities/AbbilityInputData/SBlinkInput.SBlinkInput_C|Getblink_destination_ _assblink_input) "0, 0, 0"))
            (return _returnvalue_2))))
      (:CastFailed
        ;[0.6 0 0] Error
        (Development|PrintString "[ERR] Blink cast failed" true true "(R=1.000000,G=0.051017,B=0.000000,A=1.000000)" 1e+01)
        (return false)))
    (else
      (return false))))

(fn UpdateTimers
  (params (inDelta :type Float%20%28single-precision%29))
  (bind __void_ (|CallParentFunction inDelta))
  (return __void_))