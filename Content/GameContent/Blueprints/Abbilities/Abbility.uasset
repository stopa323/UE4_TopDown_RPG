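; Ability Blueprint that gates activation on a readiness flag and a health and energy cost.
; Activate clears IsReady when IsActivateFeasible passes, without deducting any cost.
; UpdateTimers accumulates the passed delta until Cooldown is reached, then restores readiness and prints a message.
; CompareCost branches on both resources but returns only the health comparison, so energy does not affect the result.
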(fn ConstructionScript)

(fn Activate
  (params (inInputStruct :type S%20Abbility%20Input%20Object%20Reference%20%28by%20ref%29))
  (bind _outpossible (CallFunction|IsActivateFeasible inInputStruct))
  (if _outpossible
    (Variables|Default|Setis_ready_ false))
  (return _outpossible))

(fn IsActivateFeasible
  (params (inInputStruct :type S%20Abbility%20Input%20Object%20Reference%20%28by%20ref%29))
  (if (Variables|Default|Getis_ready_)
    (bind _outok (Utilities|CompareCost (Variables|/Game/GameContent/Blueprints/Abbilities/AbbilityInputData/SAbbilityInput.SAbbilityInput_C|Getcost_ inInputStruct))
      (:outExec
        (return _outok)))
    (else
      (return false))))

(fn UpdateTimers
  (params (inDelta :type Float%20%28single-precision%29))
  ;[0 0 0] if ready, dont count
  (if (Variables|Default|Getis_ready_)
    (return 0)
    (else
      (bind _output_get (Variables|Default|Settimer_ (+ inDelta (Variables|Default|Gettimer_))))
      ;[0 0 0] cooldown exceeded
      (if (>= _output_get (Variables|Default|Getcooldown_))
        (Variables|Default|Setis_ready_ true)
        (Variables|Default|Settimer_ 0.0)
        (Development|PrintString "Abbiity ready")
        (return 0)
        (else
          (return 0))))))