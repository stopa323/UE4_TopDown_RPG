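; RPGPlayerPawn is the player's pawn in an RPG, setting up its own camera and moving to destinations on request.
; On BeginPlay it spawns an RPGPlayerCamera attached to itself, then registers both with the RPGPlayerController and caches that controller.
; MovetoDestination drives AI Move To on the pawn, clearing the controller's IsMoving flag on success or failure.
; Failed camera spawns or controller casts print error messages.
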(event EventBeginPlay
  (Utilities|SpawnCamera
    (:outExec
      ;[1 1 1] move any ref creation to construction script
      (bind _asrpgplayer_controller (Utilities|Casting|CastToRPGPlayerController (Game|GetPlayerController 0))
        (:then
          (Default|OnPlayerSpawn _asrpgplayer_controller self (Variables|Global|Getcamera_))
          (Variables|Global|Setplayer_controller_ _asrpgplayer_controller))
        (:CastFailed
          (Development|PrintString "[ERR] RPGPlayerPawn::BeginPlay RPGPlayerController cast failed" true true "(R=1.000000,G=0.052581,B=0.000000,A=1.000000)" 1e+01))))))

(event EventMovetoDestination
  (params (inDestination :type Vector))
  (Utilities|MoveHandling inDestination))

(fn ConstructionScript)