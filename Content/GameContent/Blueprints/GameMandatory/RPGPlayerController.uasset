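; Player controller for a click-to-move RPG that possesses a separate camera pawn while commanding the character pawn.
; BeginPlay shows the cursor, caches the game mode, creates the game UI and spawns attribute and ability manager actors, which Tick updates.
; Move clicks place a timed indicator and send the pawn a destination message.
; Q triggers blink toward the cursor via a spawned input actor; D and I adjust health.
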(event Custom|OnPlayerSpawn
  (params (inPawnRef :type RPG%20Player%20Pawn%20Object%20Reference) (inCameraRef :type RPG%20Player%20Camera%20Object%20Reference))
  (Global|SetPawnRelatedData inPawnRef inCameraRef)
  (Pawn|Possess (Variables|Global|Getcamera_pawn_)))

(event EventBeginPlay
  (Utilities|ShowMouse
    (:outExec
      (Utilities|SetReferences
        (:outExec
          (Utilities|CreateWidgets
            (:outExec
              (Utilities|InitializeManagers))))))))

(event EventTick
  (params (DeltaSeconds :type Float%20%28single-precision%29))
  (Default|UpdateAttributes (Variables|Managers|GetAttrManager) DeltaSeconds)
  (Default|UpdateAbbilities (Variables|Managers|GetAbbilityManager) DeltaSeconds))

(event Input|ActionEvents|InputActionMoveAction
  (params (Key :type Key%20Structure :default "AnyKey"))
  (:Pressed
    (Mouse|MoveActionHandler)))

(event Input|KeyboardEvents|D
  (params (Key :type Key%20Structure :default "AnyKey"))
  (:Pressed
    (Default|DecreaseHealth (Variables|Managers|GetAttrManager) 1e+01)))

(event Input|KeyboardEvents|I
  (params (Key :type Key%20Structure :default "AnyKey"))
  (:Pressed
    (Default|IncreaseHealth (Variables|Managers|GetAttrManager) 1e+01)))

(event Input|KeyboardEvents|Q
  (params (Key :type Key%20Structure :default "AnyKey"))
  (:Pressed
    (Abbilityhandlers|BlinkHandler)))

(fn ConstructionScript)

(fn MoveActionHandler
  (Utilities|FlowControl|Sequence
    (:then_0
      (Utilities|SetMouseClickLocation))
    (:then_1
      (Utilities|SpawnMoveIndicator))
    (:then_2
      (Variables|Movement|SetbIsMoving true))
    (:then_3
      ;[1 1 1] nav invokers
      (Class|IPlayerInput|MovetoDestination(Message) (Variables|Global|Getpawn_) (Variables|Movement|Getmouse_click_location_)))))

(fn SetPawnRelatedData
  (params (inPawnRef :type RPG%20Player%20Pawn%20Object%20Reference) (inCameraRef :type RPG%20Player%20Camera%20Object%20Reference))
  (bind _output_get (Variables|Global|Setpawn_ inPawnRef))
  (bind _returnvalue (AI|GetAIController _output_get))
  (bind _asrpgplayer_aicontroller (Utilities|Casting|CastToRPGPlayerAIController _returnvalue)
    (:then
      (Variables|Global|Setpawn_controller_ _asrpgplayer_aicontroller)
      (Variables|Global|Setcamera_pawn_ inCameraRef))
    (:CastFailed
      ;[0.5 0 0] Error
      (Development|PrintString "[ERR] RPGPlayerController::SetPawnRelatedData RPGPlayerAIController cast failed" true true "(R=1.000000,G=0.000000,B=0.000000,A=1.000000)" 1e+01))))

(fn BlinkHandler
  (bind _hitresult (Game|Player|GetHitResultUnderCursorbyChannel "TraceTypeQuery3" true))
  (bind _returnvalue (Game|SpawnActorfromClass "/Game/GameContent/Blueprints/Abbilities/AbbilityInputData/SBlinkInput.SBlinkInput_C" (Math|Transform|MakeTransform "0, 0, 0" "0, 0, 0" "1,1,1") "Undefined" 0 (Math|Vector|MakeVector (.x (.location _hitresult)) (.y (.location _hitresult)) (+ (.z (.location _hitresult)) 9e+01)) (Variables|Global|Getpawn_) (Utilities|Struct|MakeSAbbilityCost (Variables|/Game/GameContent/Blueprints/Structures/Miscellaneous/SAttribute.SAttribute_C|Getcurrent_value_ (Variables|/Game/GameContent/Blueprints/PlayerCharacter/AttributeManager.AttributeManager_C|Gethealth_ (Variables|Managers|GetAttrManager))) 0.0)))
  (Default|EActivateBlink (Variables|Managers|GetAbbilityManager) _returnvalue)
  (return))