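; BP_MovingWall is an environment wall that slides continuously back and forth between two points.
; The construction script stores the placed location and sets a destination a fixed distance opposite the Cube's forward vector.
; Tick ping-pongs a normalized Timer at a rate set by Lifetime, flipping DestReached at each end.
; That Timer linearly interpolates the Scene component's world location, without sweeping.
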(event EventTick
  (params (DeltaSeconds :type Float%20%28single-precision%29))
  (if (Variables|Default|GetbDestReached_)
    (bind _output_get (Variables|Default|Settimer_ (- (Variables|Default|Gettimer_) (/ DeltaSeconds (Variables|Default|Getlifetime_)))))
    (if (<= _output_get 0.0)
      (Variables|Default|SetbDestReached_ false))
    (else
      (bind _output_get_2 (Variables|Default|Settimer_ (+ (Variables|Default|Gettimer_) (/ DeltaSeconds (Variables|Default|Getlifetime_)))))
      (if (>= _output_get_2 1.0)
        (Variables|Default|SetbDestReached_ true))))
  (Transformation|SetWorldLocation (Variables|Default|GetScene) (Math|Vector|Lerp(Vector) (Variables|Default|Getinitial_location_) (Variables|Default|Getdestination_) (Variables|Default|Gettimer_)) false false))

(fn ConstructionScript
  (bind _output_get (Variables|Default|Setinitial_location_ (Transformation|GetActorLocation)))
  (Variables|Default|Setdestination_ (- _output_get (* (Math|Vector|GetForwardVector (Variables|Default|GetCube)) 5e+02))))